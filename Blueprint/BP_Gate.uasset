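; Gate actor that raises or lowers its static mesh with a scraping stone sound, triggered by open and close events.
; A single timeline plays forward to open and in reverse to close, setting the mesh's absolute world Z from its height track.
; Each event spawns the sound at the actor's location.
; When the timeline finishes, it stops the opening sound if valid, otherwise the closing one.
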(event Custom|GateOpen_Event
  (bind _staticmesh (Variables|Default|GetStaticMesh))
  (bind _returnvalue (Transformation|GetWorldLocation _staticmesh))
  ;[1 1 1] Gate Open and Close
  (bind _returnvalue_2 (Audio|SpawnSoundatLocation "/Game/Audio/scraping-stone.scraping-stone" (Transformation|GetActorLocation) "0, 0, 0" 1.0 1.0 0.0 0 0))
  (bind _zheight (Timeline|GateOpen_Timeline PlayFromStart)
    (:Update
      (Transformation|SetWorldLocation _staticmesh (Math|Vector|MakeVector (.x _returnvalue) (.y _returnvalue) _zheight) false false))
    (:Finished
      (Utilities|IsValid _returnvalue_2
        (:Is%20Valid
          (Audio|Components|Audio|Stop _returnvalue_2))
        (:Is%20Not%20Valid
          (Utilities|IsValid (stale Custom|GateClose_Event _returnvalue_2)
            (:Is%20Valid
              (Audio|Components|Audio|Stop (stale Custom|GateClose_Event _returnvalue_2)))))))))

(event Custom|GateClose_Event
  (bind _staticmesh (Variables|Default|GetStaticMesh))
  (bind _returnvalue (Transformation|GetWorldLocation _staticmesh))
  ;[1 1 1] Gate Open and Close
  (bind _returnvalue_2 (Audio|SpawnSoundatLocation "/Game/Audio/scraping-stone.scraping-stone" (Transformation|GetActorLocation) "0, 0, 0" 1.0 1.0 0.0 0 0))
  (bind _zheight (Timeline|GateOpen_Timeline ReverseFromEnd)
    (:Update
      (Transformation|SetWorldLocation _staticmesh (Math|Vector|MakeVector (.x _returnvalue) (.y _returnvalue) _zheight) false false))
    (:Finished
      (Utilities|IsValid (stale Custom|GateOpen_Event _returnvalue_2)
        (:Is%20Valid
          (Audio|Components|Audio|Stop (stale Custom|GateOpen_Event _returnvalue_2)))
        (:Is%20Not%20Valid
          (Utilities|IsValid _returnvalue_2
            (:Is%20Valid
              (Audio|Components|Audio|Stop _returnvalue_2))))))))

(fn ConstructionScript)
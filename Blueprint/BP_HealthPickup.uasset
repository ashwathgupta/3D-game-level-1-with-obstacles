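; BP_HealthPickup is a pickup actor that heals the player on touch.
; BeginPlay caches the first player's BP_ThirdPersonCharacter as a reference.
; When that character overlaps the Sphere, it adds HealAmount to CurrentHealth, clamped between zero and a hardcoded maximum, plays a pop sound at its location and destroys itself.
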(event OnComponentBeginOverlap(Sphere)
  (params (OverlappedComponent :type Primitive%20Component%20Object%20Reference) (OtherActor :type Actor%20Object%20Reference) (OtherComp :type Primitive%20Component%20Object%20Reference) (OtherBodyIndex :type Integer) (bFromSweep :type Boolean) (SweepResult :type Hit%20Result%20Structure%20%28by%20ref%29))
  (bind _player_ref (Variables|Default|GetPlayer%20Ref))
  ;[1 1 1] Pickup
  (if (== OtherActor (Variables|Default|GetPlayer%20Ref))
    (Variables|/Game/Blueprint/BP_ThirdPersonCharacter.BP_ThirdPersonCharacter_C|SetCurrentHealth _player_ref (Math|Float|Clamp(Float) (+ (Variables|/Game/Blueprint/BP_ThirdPersonCharacter.BP_ThirdPersonCharacter_C|GetCurrentHealth _player_ref) (Variables|Default|GetHealAmount)) 0.0 1e+02))
    (Audio|PlaySoundatLocation "/Game/Audio/cartoon-pop.cartoon-pop" (Transformation|GetActorLocation) "0, 0, 0" 1.0 1.0 0.0 0 0 0 0)
    (Actor|DestroyActor)))

(event EventBeginPlay
  ;[1 1 1] Create player ref
  (bind _asbp_third_person_character (Utilities|Casting|CastToBP_ThirdPersonCharacter (Game|GetPlayerCharacter 0)))
  (Variables|Default|SetPlayer%20Ref _asbp_third_person_character))

(fn ConstructionScript)
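; BP_Button is a pressure button that opens and closes a linked gate when the player steps on or off it.
; Sphere overlaps with the cached player character play or reverse a timeline that moves the mesh along Z.
; When the timeline finishes in either direction, a sound plays and the ButtonDown flag selects GateOpenEvent, or GateCloseEvent after a delay, on BPGateRef.
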(event OnComponentBeginOverlap(Sphere)
  (params (OverlappedComponent :type Primitive%20Component%20Object%20Reference) (OtherActor :type Actor%20Object%20Reference) (OtherComp :type Primitive%20Component%20Object%20Reference) (OtherBodyIndex :type Integer) (bFromSweep :type Boolean) (SweepResult :type Hit%20Result%20Structure%20%28by%20ref%29))
  (bind _staticmesh (Variables|Default|GetStaticMesh))
  (bind _bp_gateref (Variables|Default|GetBP_GateRef))
  (bind _relativelocation (Variables|/Script/Engine.SceneComponent|GetRelativeLocation _staticmesh))
  ;[1 1 1] Button Down
  (if (== OtherActor (Variables|Default|GetPlayer%20Ref))
    (Variables|Default|SetbButtonDown true)
    (bind _z_height (Timeline|ButtonDown_Timeline Play)
      (:Update
        (Transformation|SetRelativeLocation _staticmesh (Math|Vector|MakeVector (.x _relativelocation) (.y _relativelocation) _z_height) false false))
      (:Finished
        (Audio|PlaySoundatLocation 0 (Transformation|GetActorLocation) "0, 0, 0" 1.0 1.0 0.0 0 0 0 0)
        ;[1 1 1] Gate open and close
        (if (Variables|Default|GetbButtonDown)
          (Utilities|IsValid _bp_gateref
            (:Is%20Valid
              (Default|GateOpenEvent _bp_gateref)))
          (else
            (Utilities|IsValid _bp_gateref
              (:Is%20Valid
                (Utilities|FlowControl|Delay (Variables|Default|GetDelayTime))
                (Default|GateCloseEvent _bp_gateref)))))))))

(event OnComponentEndOverlap(Sphere)
  (params (OverlappedComponent :type Primitive%20Component%20Object%20Reference) (OtherActor :type Actor%20Object%20Reference) (OtherComp :type Primitive%20Component%20Object%20Reference) (OtherBodyIndex :type Integer))
  (bind _staticmesh (Variables|Default|GetStaticMesh))
  (bind _bp_gateref (Variables|Default|GetBP_GateRef))
  (bind _relativelocation (Variables|/Script/Engine.SceneComponent|GetRelativeLocation _staticmesh))
  ;[1 1 1] Button Up
  (if (== OtherActor (Variables|Default|GetPlayer%20Ref))
    (Variables|Default|SetbButtonDown false)
    ;[1 1 1] Button Down
    (bind _z_height (Timeline|ButtonDown_Timeline Reverse)
      (:Update
        (Transformation|SetRelativeLocation _staticmesh (Math|Vector|MakeVector (.x _relativelocation) (.y _relativelocation) _z_height) false false))
      (:Finished
        (Audio|PlaySoundatLocation 0 (Transformation|GetActorLocation) "0, 0, 0" 1.0 1.0 0.0 0 0 0 0)
        ;[1 1 1] Gate open and close
        (if (Variables|Default|GetbButtonDown)
          (Utilities|IsValid _bp_gateref
            (:Is%20Valid
              (Default|GateOpenEvent _bp_gateref)))
          (else
            (Utilities|IsValid _bp_gateref
              (:Is%20Valid
                (Utilities|FlowControl|Delay (Variables|Default|GetDelayTime))
                (Default|GateCloseEvent _bp_gateref)))))))))

(event EventBeginPlay
  ;[1 1 1] Create Player reference
  (bind _asbp_third_person_character (Utilities|Casting|CastToBP_ThirdPersonCharacter (Game|GetPlayerCharacter 0)))
  (Variables|Default|SetPlayer%20Ref _asbp_third_person_character))

(fn ConstructionScript)
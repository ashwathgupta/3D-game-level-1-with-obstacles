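; BP_FIreSpurt is a fire trap that burns the player while they stand inside its trigger box.
; On overlap it waits briefly, then shows the particle effect and plays a flamethrower sound at its location.
; While the flames are visible and the player overlaps the box, Tick applies damage at one-second intervals using a DoOnce reset after a delay.
; Leaving the box hides the flames and stops the sound after a delay.
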(event OnComponentBeginOverlap(Box)
  (params (OverlappedComponent :type Primitive%20Component%20Object%20Reference) (OtherActor :type Actor%20Object%20Reference) (OtherComp :type Primitive%20Component%20Object%20Reference) (OtherBodyIndex :type Integer) (bFromSweep :type Boolean) (SweepResult :type Hit%20Result%20Structure%20%28by%20ref%29))
  ;[1 1 1] Activate Fire
  (if (== OtherActor (Variables|Default|GetPlayer%20Ref))
    (Utilities|FlowControl|Delay 0.25)
    (Rendering|SetVisibility (Variables|Default|GetParticleSystem) true false)
    (bind _returnvalue (Audio|SpawnSoundatLocation "/Game/Audio/flamethrower-sound-effect-203135.flamethrower-sound-effect-203135" (Transformation|GetActorLocation) "0, 0, 0" 1.0 1.0 0.0 0 0))))

(event OnComponentEndOverlap(Box)
  (params (OverlappedComponent :type Primitive%20Component%20Object%20Reference) (OtherActor :type Actor%20Object%20Reference) (OtherComp :type Primitive%20Component%20Object%20Reference) (OtherBodyIndex :type Integer))
  ;[1 1 1] Deactivate Fire
  (if (== OtherActor (Variables|Default|GetPlayer%20Ref))
    (if true
      (Utilities|FlowControl|Delay 1.0)
      (Rendering|SetVisibility (Variables|Default|GetParticleSystem) false false)
      (Audio|Components|Audio|Stop (stale OnComponentBeginOverlap(Box) _returnvalue)))))

(event EventBeginPlay
  ;[1 1 1] Player Ref
  (bind _asbp_third_person_character (Utilities|Casting|CastToBP_ThirdPersonCharacter (Game|GetPlayerCharacter 0)))
  (Variables|Default|SetPlayer%20Ref _asbp_third_person_character))

(event EventTick
  (params (DeltaSeconds :type Float%20%28single-precision%29))
  ;[1 1 1] Apply Damage
  (if (Rendering|IsVisible (Variables|Default|GetParticleSystem))
    (if (Collision|IsOverlappingActor (Variables|Default|GetBox) (Variables|Default|GetPlayer%20Ref) :!class /Script/Engine.PrimitiveComponent)
      (Utilities|FlowControl|DoOnce false :!label _label
        (:Completed
          (Game|Damage|ApplyDamage (Variables|Default|GetPlayer%20Ref) 1e+01 0 0)
          (Utilities|FlowControl|Delay 1.0)
          (goto _label Reset))))))

(fn ConstructionScript)
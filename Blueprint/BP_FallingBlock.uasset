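; BP_FallingBlock is a trap block that drops when the player enters its Box trigger, then rises again.
; BeginPlay caches the third-person character, and a Box overlap by it starts the BlockFall timeline after a short delay.
; When the fall ends, a thud sound plays and, after a pause, the BlockRise timeline runs.
; Both timelines set the static mesh's absolute world Z, keeping X and Y.
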(event OnComponentBeginOverlap(Box)
  (params (OverlappedComponent :type Primitive%20Component%20Object%20Reference) (OtherActor :type Actor%20Object%20Reference) (OtherComp :type Primitive%20Component%20Object%20Reference) (OtherBodyIndex :type Integer) (bFromSweep :type Boolean) (SweepResult :type Hit%20Result%20Structure%20%28by%20ref%29))
  (bind _staticmesh (Variables|Default|GetStaticMesh))
  (bind _staticmesh_2 (Variables|Default|GetStaticMesh))
  (bind _returnvalue (Transformation|GetWorldLocation _staticmesh))
  (bind _returnvalue_2 (Transformation|GetWorldLocation _staticmesh_2))
  ;[1 1 1] BlockFall
  (if (== OtherActor (Variables|Default|GetPlayerRef))
    (Utilities|FlowControl|Delay 0.2)
    (bind _zheight (Timeline|BlockFall PlayFromStart)
      (:Update
        (Transformation|SetWorldLocation _staticmesh_2 (Math|Vector|MakeVector (.x _returnvalue_2) (.y _returnvalue_2) _zheight) false false))
      (:Finished
        (Audio|PlaySoundatLocation "/Game/Audio/big-thud.big-thud" (Transformation|GetActorLocation) "0, 0, 0" 1.0 1.0 0.0 0 0 0 0)
        ;[1 1 1] Block rise
        (Utilities|FlowControl|Delay 1.0)
        (bind _zheight_2 (Timeline|BlockRise PlayFromStart)
          (:Update
            (Transformation|SetWorldLocation _staticmesh (Math|Vector|MakeVector (.x _returnvalue) (.y _returnvalue) _zheight_2) false false)))))))

(event EventBeginPlay
  ;[1 1 1] Create player reference
  (bind _asbp_third_person_character (Utilities|Casting|CastToBP_ThirdPersonCharacter (Game|GetPlayerCharacter 0)))
  (Variables|Default|SetPlayerRef _asbp_third_person_character))

(event Collision|EventActorBeginOverlap
  (params (OtherActor :type Actor%20Object%20Reference)))

(event EventTick
  (params (DeltaSeconds :type Float%20%28single-precision%29)))

(fn ConstructionScript)
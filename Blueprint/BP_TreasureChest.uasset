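; BP_TreasureChest is a chest that opens once when the player character walks into its Box trigger and pops out a health pickup.
; BeginPlay caches the player reference, which the overlap checks before a DoOnce plays a timeline that rotates the lid's roll.
; When the timeline finishes, SpawnItems spawns a BP_HealthPickup at SpawnPoint, enables physics on its mesh and launches it with an impulse.
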(event OnComponentBeginOverlap(Box)
  (params (OverlappedComponent :type Primitive%20Component%20Object%20Reference) (OtherActor :type Actor%20Object%20Reference) (OtherComp :type Primitive%20Component%20Object%20Reference) (OtherBodyIndex :type Integer) (bFromSweep :type Boolean) (SweepResult :type Hit%20Result%20Structure%20%28by%20ref%29))
  (bind _lid (Variables|Default|GetLid))
  (bind _relativerotation (Variables|/Script/Engine.SceneComponent|GetRelativeRotation _lid))
  ;[1 1 1] Lid Open
  (if (== OtherActor (Variables|Default|GetPlayer%20Ref))
    (Utilities|FlowControl|DoOnce false
      (:Completed
        (bind _xrotation (Timeline|OpenLid_Timeline Play)
          (:Update
            (Transformation|SetRelativeRotation _lid (Math|Rotator|MakeRotator _xrotation (.pitch _relativerotation) (.yaw _relativerotation)) false false))
          (:Finished
            ;[1 1 1] Spawn item
            (CallFunction|SpawnItems)))))))

(event Custom|SpawnItems
  ;[1 1 1] Spawn item
  (bind _returnvalue (Game|SpawnActorfromClass "/Game/Blueprint/BP_HealthPickup.BP_HealthPickup_C" (Transformation|GetWorldTransform (Variables|Default|GetSpawnPoint)) "Undefined" "MultiplyWithRoot" 0 0))
  (Physics|SetSimulatePhysics (Variables|/Game/Blueprint/BP_HealthPickup.BP_HealthPickup_C|GetStaticMesh _returnvalue) true)
  (Physics|AddImpulseatLocation (Variables|/Game/Blueprint/BP_HealthPickup.BP_HealthPickup_C|GetStaticMesh _returnvalue) "0.000000,1000.000000,5000.000000" (Transformation|GetActorLocation _returnvalue) "None"))

(event EventBeginPlay
  ;[1 1 1] Create player reference
  (bind _asbp_third_person_character (Utilities|Casting|CastToBP_ThirdPersonCharacter (Game|GetPlayerCharacter 0)))
  (Variables|Default|SetPlayer%20Ref _asbp_third_person_character))

(fn ConstructionScript)